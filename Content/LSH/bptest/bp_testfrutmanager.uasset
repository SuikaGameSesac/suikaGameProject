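; Test fruit manager actor that spawns leveled Bp_testactor fruits, apparently for a merge-style mechanic.
; From BeginPlay, it loops every second, spawning a level 0 fruit at a random point 100 units from itself.
; Each fruit receives its level and a manager reference.
; The hit event spawns a next-level fruit at the hit location, ignoring repeats of the last recorded location to avoid duplicate spawns.
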(event `self.ReceiveBeginPlay`
  (`KismetSystemLibrary.Delay` 1.0 :!label _label)
  (`self.create fruit` (+ (* (`KismetMathLibrary.RandomUnitVector`) 100) (`self.K2_GetActorLocation`)))
  (goto _label))

(event `create fruit`
  (params (createLocation :type "Vector Structure") (level :type Integer))
  (bind _returnvalue (`|SpawnActorFromClass` "/Game/LSH/bptest/bp_testactor.bp_testactor_C" (`KismetMathLibrary.MakeTransform` createLocation) "Undefined" "MultiplyWithRoot" null null))
  (set `/Game/LSH/bptest/bp_testactor.manager` self _returnvalue)
  (set `/Game/LSH/bptest/bp_testactor.level` level _returnvalue))

(event `afterHitevent`
  (params (hitLocation :type "Vector Structure") (level :type Integer))
  (if (not (== hitLocation (`self.pastCreateLocation`)))
    (set `self.pastCreateLocation` hitLocation)
    (bind _result (`/Engine/EditorBlueprintResources/StandardMacros.IncrementInt` level)
      (:`  `
        (`self.create fruit` hitLocation _result)))))

(fn `UserConstructionScript`)