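; Test fruit actor for a merge game: a leveled sphere that merges on hitting another of the same level.
; SetShow runs a tick after BeginPlay, scaling the actor and tinting the sphere by powers of two of Level.
; A matching hit reports location and level to Manager once, then destroys itself next tick.
; Tick locks the Y position, draws the level as debug text and fixes the widget's world yaw.
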(event `self.ReceiveBeginPlay`
  (`KismetSystemLibrary.DelayUntilNextTick`)
  (`self.setShow`))

(event `self.ReceiveTick`
  (params (DeltaSeconds :type "Float (single-precision)"))
  (bind (_returnvalue_x _returnvalue_y _returnvalue_z) (`KismetMathLibrary.BreakVector` (`self.K2_GetActorLocation`)))
  (bind _widget (`self.Widget`))
  (bind (_returnvalue_roll _returnvalue_pitch) (`KismetMathLibrary.BreakRotator` (`SceneComponent.K2_GetComponentRotation` _widget)))
  ;[1 1 1] 과일의 y축 고정
  (`self.K2_SetActorLocation` (`KismetMathLibrary.MakeVector` _returnvalue_x 0.0 _returnvalue_z))
  (`KismetSystemLibrary.DrawDebugString` (`self.K2_GetActorLocation`) (`KismetStringLibrary.Conv_IntToString` (`self.level`)) null)
  (`SceneComponent.K2_SetWorldRotation` _widget (`KismetMathLibrary.MakeRotator` _returnvalue_roll _returnvalue_pitch 90.0) false false))

(event `self.ReceiveHit`
  (params (MyComp :type "PrimitiveComponent Object Reference") (Other :type "Actor Object Reference") (OtherComp :type "PrimitiveComponent Object Reference") (bSelfMoved :type Boolean) (HitLocation :type "Vector Structure") (HitNormal :type "Vector Structure") (NormalImpulse :type "Vector Structure") (Hit :type "HitResult Structure (by ref)"))
  (bind _asbp_testactor (cast `/Game/LSH/bptest/bp_testactor` Other))
  (if (== (`/Game/LSH/bptest/bp_testactor.level` _asbp_testactor) (`self.level`))
    (`/Engine/EditorBlueprintResources/StandardMacros.DoOnce` false
      (:`Completed`
        (`KismetSystemLibrary.PrintString` (`KismetSystemLibrary.GetDisplayName` self))
        (`/Game/LSH/bptest/bp_testfrutmanager.afterHitevent` (`self.manager`) HitLocation (`self.level`))
        (`KismetSystemLibrary.DelayUntilNextTick`)
        (`self.K2_DestroyActor`)))))

(fn `setShow`
  (`self.SetActorScale3D` (* (`KismetMathLibrary.MakeVector` 1.0 1.0 1.0) (+ (* (`KismetMathLibrary.MultiplyMultiply_FloatFloat` 2.0 (`KismetMathLibrary.Conv_IntToDouble` (`self.level`))) 0.1) 1.0)))
  (`MeshComponent.SetVectorParameterValueOnMaterials` (`self.Sphere1`) "Color" (+ (`KismetMathLibrary.MakeVector` 0.0) (* (`KismetMathLibrary.MultiplyMultiply_FloatFloat` 2.0 (`KismetMathLibrary.Conv_IntToDouble` (`self.level`))) 0.05))))

(fn `UserConstructionScript`)